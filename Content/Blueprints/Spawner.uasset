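; Spawner actor that periodically spawns actors of a configurable class around every player.
; Tick counts down a random timeout, capped by MaxSeconds and re-rolled through NewTimeout at BeginPlay and after each expiry.
; On expiry it finds all PlayerBase actors and spawns one at a random point in a SpawnSize box around each, adjusting for collision but always spawning.
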(event `self.ReceiveBeginPlay`
  (`self.NewTimeout`))

(event `self.ReceiveTick`
  (params (DeltaSeconds :type "Float (single-precision)"))
  ;[1 1 1] Spawn targets round the player
  (bind _output_get (set `self.Timeout` (- (`self.Timeout`) DeltaSeconds)))
  (if (<= _output_get 0.0)
    (`self.NewTimeout`)
    (bind _outactors (`GameplayStatics.GetAllActorsOfClass` "/Script/UECPPArcade.PlayerBase"))
    (for _array_element _outactors
      (`|SpawnActorFromClass` (`self.Actor`) (`KismetMathLibrary.MakeTransform` (`KismetMathLibrary.RandomPointInBoundingBox` (`self.K2_GetActorLocation` _array_element) (* (`KismetMathLibrary.Vector_One`) (`self.SpawnSize`)))) "AdjustIfPossibleButAlwaysSpawn" "OverrideRootScale" null null))))

(fn `NewTimeout`
  (set `self.Timeout` (* (`KismetMathLibrary.RandomFloat`) (`self.MaxSeconds`))))

(fn `UserConstructionScript`)